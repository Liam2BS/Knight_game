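; GM_KnightGame is the game mode for the Knight game, managing enemy spawn timing and the live enemy count.
; RegisterSpawner stores the spawner and starts a looping timer at the EnemyPerSeconds rate through a created delegate, whose target function is not shown.
; AddOneEnemy and RemoveOneEnemy maintain the count, which GetEnemyCount returns and CanSpawnOneEnemy checks against MaxEnemyCount.
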(event `/Game/Cass/GameSettings/BPI_GameModeMP.RegisterSpawner`
  (params (NewSpawner :type "/Game/Cass/GameSettings/NEEDintoMAP/BP_Spawner Object Reference"))
  ;[0.06424 0.06424 0.06424] Get ref spawner and make spawner enemy
  (set `self.Spawner` NewSpawner)
  (`KismetSystemLibrary.K2_SetTimerDelegate` (`|CreateDelegate` (`self.Spawner`) :!event `SpawnOneEnemy`) (/ 1.0 (`self.EnemyPerSeconds`)) true))

(event `/Game/Cass/GameSettings/BPI_GameModeMP.AddOneEnemy`
  ;[0.06424 0.06424 0.06424] Enemy Count
  (`/Engine/EditorBlueprintResources/StandardMacros.IncrementInt` (`self.CurrentEnemyCount`)))

(event `/Game/Cass/GameSettings/BPI_GameModeMP.RemoveOneEnemy`
  ;[0.06424 0.06424 0.06424] Enemy Count
  (`/Engine/EditorBlueprintResources/StandardMacros.DecrementInt` (`self.CurrentEnemyCount`)))

(fn `CanSpawnOneEnemy`
  (returns (bResult :type Boolean))
  (return (< (`self.CurrentEnemyCount`) (`self.MaxEnemyCount`))))

(fn `GetEnemyCount`
  (returns (Count :type Integer))
  (return (`self.CurrentEnemyCount`)))

(fn `UserConstructionScript`)