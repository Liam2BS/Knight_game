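; BP_Spawner is a map-placed spawner that creates dark spider enemies inside a box zone.
; On BeginPlay it registers itself with the game mode through a message call.
; When SpawnOneEnemy fires, it asks the game mode whether another enemy is allowed, spawns one at a random point within EnnemiesSpawnZone, then reports the addition back to the game mode.
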(event `self.ReceiveBeginPlay`
  ;[0.06424 0.06424 0.06424] Send his reference to game mode
  (message `/Game/Cass/GameSettings/BPI_GameModeMP.RegisterSpawner` (`GameplayStatics.GetGameMode`) self))

(event `SpawnOneEnemy`
  (bind _ennemiesspawnzone (`self.EnnemiesSpawnZone`))
  ;[0.06424 0.06424 0.06424] Spawn Enemy
  (bind _bresult (message `/Game/Cass/GameSettings/BPI_GameModeMP.CanSpawnOneEnemy` (`GameplayStatics.GetGameMode`)))
  (if _bresult
    (`AIBlueprintHelperLibrary.SpawnAIFromClass` "/Game/Cass/Spider/BP/Chara_DarkSpider.Chara_DarkSpider_C" null (`KismetMathLibrary.RandomPointInBoundingBox` (`SceneComponent.K2_GetComponentLocation` _ennemiesspawnzone) (`BoxComponent.GetScaledBoxExtent` _ennemiesspawnzone)) (struct) false null)
    (message `/Game/Cass/GameSettings/BPI_GameModeMP.AddOneEnemy` (`GameplayStatics.GetGameMode`))))

(fn `UserConstructionScript`)