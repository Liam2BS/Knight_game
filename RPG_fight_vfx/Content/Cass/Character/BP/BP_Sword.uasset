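; BP_Sword is the player's melee weapon actor that deals damage to things it touches during an attack.
; On BeginPlay it caches the player pawn as BP_Character.
; On actor overlap, if that character is attacking, it sends AffectHealth with its damage amount to actors implementing BPI_Damageable, skipping any tagged Player.
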(event `self.ReceiveBeginPlay`
  ;[0.06424 0.06424 0.06424] Cast Player Character
  (bind _asbp_character (cast `/Game/Cass/Character/BP/BP_Character` (`GameplayStatics.GetPlayerPawn` 0)))
  (bind _output_get (set `self.As CPlayer Character` _asbp_character)))

(event `self.ReceiveActorBeginOverlap`
  (params (OtherActor :type "Actor Object Reference"))
  ;[0.06424 0.06424 0.06424] Check sword overlap a spider
  (if (and (`/Game/Cass/Character/BP/BP_Character.IsAttacking` (stale `self.ReceiveBeginPlay` _output_get)) (`KismetSystemLibrary.DoesImplementInterface` OtherActor "/Game/Cass/GameSettings/BPI_Damageable.BPI_Damageable_C"))
    (if (not (`self.ActorHasTag` OtherActor "Player"))
      (message `/Game/Cass/GameSettings/BPI_Damageable.AffectHealth` OtherActor (`self.DamageAmount`)))))

(fn `UserConstructionScript`)